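; BP_PlayerBase is a player base Blueprint that moves by physics forces and looks around through controller input.
; MoveForward and MoveRight pass the camera's forward or right vector and the axis value to GetMovementDirection, which scales them by MoveSpeed.
; The result is applied to the StaticMesh as a mass-independent acceleration via AddForce.
; Turn and LookUp feed controller yaw and pitch.
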(event EventBeginPlay)

(event EventTick
  (params (DeltaSeconds :type Float%20%28single-precision%29)))

(event Input|AxisEvents|InputAxisMoveForward
  (params (AxisValue :type Float%20%28single-precision%29))
  (Physics|AddForce (Variables|Default|GetStaticMesh) (CallFunction|GetMovementDirection (Math|Vector|GetForwardVector (Variables|Default|GetCamera)) (Input|AxisValues|GetMoveForward)) "None" true))

(event Input|AxisEvents|InputAxisMoveRight
  (params (AxisValue :type Float%20%28single-precision%29))
  (Physics|AddForce (Variables|Default|GetStaticMesh) (CallFunction|GetMovementDirection (Math|Vector|GetRightVector (Variables|Default|GetCamera)) (Input|AxisValues|GetMoveRight)) "None" true))

(event Input|AxisEvents|InputAxisTurn
  (params (AxisValue :type Float%20%28single-precision%29))
  (Pawn|Input|AddControllerYawInput AxisValue))

(event Input|AxisEvents|InputAxisLookUp
  (params (AxisValue :type Float%20%28single-precision%29))
  (Pawn|Input|AddControllerPitchInput AxisValue))

(fn ConstructionScript)

(fn GetMovementDirection
  (params (InputDirection :type Vector) (MoveInputAxis :type Float%20%28single-precision%29))
  (return (* (* InputDirection MoveInputAxis) (Variables|Default|GetMoveSpeed))))